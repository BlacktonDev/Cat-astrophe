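; Base enemy character that sets its walk speed and health on spawn, shows health as text, and destroys itself when damage depletes it.
; Overlapping the HitRange sphere starts an endless cooldown Delay loop that damages the player while the Hiting flag is set.
; End overlap only clears that flag, leaving the loop running.
; GetAffination reports affiliation; AI movement and sphere-radius nodes are unconnected.
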(event OnComponentBeginOverlap(HitRange)
  (params (OverlappedComponent :type Primitive%20Component%20Object%20Reference) (OtherActor :type Actor%20Object%20Reference) (OtherComp :type Primitive%20Component%20Object%20Reference) (OtherBodyIndex :type Integer) (bFromSweep :type Boolean) (SweepResult :type Hit%20Result%20Structure%20%28by%20ref%29))
  ;[1 1 1] Aplica daño con cooldown
  (bind _output_get (Variables|Default|SetHiting true))
  (Utilities|FlowControl|Delay (Variables|Default|GetCooldown) :!label _label)
  (CallFunction|MakeDamage OtherActor _output_get)
  (goto _label))

(event OnComponentEndOverlap(HitRange)
  (params (OverlappedComponent :type Primitive%20Component%20Object%20Reference) (OtherActor :type Actor%20Object%20Reference) (OtherComp :type Primitive%20Component%20Object%20Reference) (OtherBodyIndex :type Integer))
  ;[1 1 1] Detiene el ataque
  (Variables|Default|SetHiting false))

(event EventBeginPlay
  ;[1 1 1] inicializa atributos del enemy
  (Variables|/Script/Engine.CharacterMovementComponent|SetMaxWalkSpeed (Variables|Character|GetCharacterMovement) (* (Variables|Default|GetSpeed) 1e+02))
  (bind _output_get (Variables|Default|SetCurrentHealt (Variables|Default|GetMaxHealt)))
  (Rendering|Components|TextRender|SetText (Variables|Default|GetHP) (Utilities|Text|ToText(Float) _output_get "HalfToEven")))

(event Collision|EventActorBeginOverlap
  (params (OtherActor :type Actor%20Object%20Reference)))

(event EventTick
  (params (DeltaSeconds :type Float%20%28single-precision%29)))

(event Game|Damage|EventAnyDamage
  (params (Damage :type Float%20%28single-precision%29) (DamageType :type Damage%20Type%20Object%20Reference) (InstigatedBy :type Controller%20Object%20Reference) (DamageCauser :type Actor%20Object%20Reference))
  ;[1 1 1] Aplica daño al enemigo
  ;[1 1 1] Si HP <= 0 destruye al actor, sino atualiza la vida del enemigo
  (bind _output_get (Variables|Default|SetCurrentHealt (Math|Float|Clamp(Float) (- (Variables|Default|GetCurrentHealt) Damage) 0.0 (Variables|Default|GetMaxHealt))))
  (if (<= _output_get 0.0)
    (Actor|DestroyActor)
    (else
      (Rendering|Components|TextRender|SetText (Variables|Default|GetHP) (Utilities|Text|ToText(Float) _output_get "HalfToEven")))))

(fn ConstructionScript)

(fn MakeDamage
  (params (OtherObject :type Object%20Object%20Reference) (IsOverlapping :type Boolean))
  (bind _returnvalue (Game|GetPlayerCharacter 0))
  ;[1 1 1] Mientras se detecte al player y siga en el rango de ataque, aplicará daño
  (if IsOverlapping
    (if (== OtherObject _returnvalue)
      (Game|Damage|ApplyDamage _returnvalue (Variables|Default|GetDamage) 0 self))))

(fn GetAffination
  (return (Variables|Default|GetAffiliation) true))