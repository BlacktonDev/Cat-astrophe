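; Parent Blueprint for basic enemy characters, providing health, movement speed and melee attacks against the player.
; BeginPlay sets walk speed and fills ACHealth, while AnyDamage clamps health, refreshes the HP text and destroys the enemy at zero.
; HitRange overlap starts an endless cooldown loop calling MakeDamage, which plays the attack montage and damages the player while IsHiting is set.
; GetAffination reports affiliation; AI movement, random material and range-radius nodes are unconnected.
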(event OnComponentBeginOverlap(HitRange)
  (params (OverlappedComponent :type Primitive%20Component%20Object%20Reference) (OtherActor :type Actor%20Object%20Reference) (OtherComp :type Primitive%20Component%20Object%20Reference) (OtherBodyIndex :type Integer) (bFromSweep :type Boolean) (SweepResult :type Hit%20Result%20Structure%20%28by%20ref%29))
  (Development|PrintString "Hello")
  (bind _output_get (Variables|Default|SetisHiting true))
  (Utilities|FlowControl|Delay (Variables|Default|Getcooldown) :!label _label)
  (CallFunction|MakeDamage (Variables|Default|GetDamage) OtherActor _output_get)
  (goto _label))

(event OnComponentEndOverlap(HitRange)
  (params (OverlappedComponent :type Primitive%20Component%20Object%20Reference) (OtherActor :type Actor%20Object%20Reference) (OtherComp :type Primitive%20Component%20Object%20Reference) (OtherBodyIndex :type Integer))
  (Variables|Default|SetisHiting false))

(event EventBeginPlay
  (bind _ac_health (Variables|Default|GetAC_Health))
  ;[1 1 1] inicializa atributos del enemy
  (Variables|/Script/Engine.CharacterMovementComponent|SetMaxWalkSpeed (Variables|Character|GetCharacterMovement) (* (Variables|Default|GetSpeed) 1e+02))
  (bind _output_get (Variables|/Game/Renato/ZombieSpawner/AC_Health.AC_Health_C|SetCurrentHealth _ac_health (Variables|/Game/Renato/ZombieSpawner/AC_Health.AC_Health_C|GetMaxHealth _ac_health)))
  (Rendering|Components|TextRender|SetText (Variables|Default|GetHP) (Utilities|Text|ToText(Float) _output_get "HalfToEven")))

(event Collision|EventActorBeginOverlap
  (params (OtherActor :type Actor%20Object%20Reference)))

(event EventTick
  (params (DeltaSeconds :type Float%20%28single-precision%29)))

(event Game|Damage|EventAnyDamage
  (params (Damage :type Float%20%28single-precision%29) (DamageType :type Damage%20Type%20Object%20Reference) (InstigatedBy :type Controller%20Object%20Reference) (DamageCauser :type Actor%20Object%20Reference))
  (bind _ac_health (Variables|Default|GetAC_Health))
  ;[1 1 1] Aplica daño al enemigo
  ;[1 1 1] Si HP <= 0 destruye al actor, sino atualiza la vida del enemigo
  (bind _output_get (Variables|/Game/Renato/ZombieSpawner/AC_Health.AC_Health_C|SetCurrentHealth _ac_health (Math|Float|Clamp(Float) (- (Variables|/Game/Renato/ZombieSpawner/AC_Health.AC_Health_C|GetCurrentHealth _ac_health) Damage) 0.0 (Variables|/Game/Renato/ZombieSpawner/AC_Health.AC_Health_C|GetMaxHealth _ac_health))))
  (if (<= _output_get 0.0)
    (Actor|DestroyActor)
    (else
      (Rendering|Components|TextRender|SetText (Variables|Default|GetHP) (Utilities|Text|ToText(Float) _output_get "HalfToEven")))))

(fn ConstructionScript)

(fn MakeDamage
  (params (Damage :type Float%20%28double-precision%29) (B :type Object%20Object%20Reference) (Condition :type Boolean))
  (bind _returnvalue (Game|GetPlayerCharacter 0))
  (if Condition
    (if (== _returnvalue B)
      (Animation|PlayAnimMontage "/Game/Ricardo/NPC/models/BaseCatEnemy/Animations/Attack_Montage.Attack_Montage" 1.0 "None")
      (Game|Damage|ApplyDamage _returnvalue Damage 0 self))))

(fn GetAffination
  (return (Variables|Default|GetAffiliation) true))