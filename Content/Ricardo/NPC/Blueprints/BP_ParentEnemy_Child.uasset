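; BP_ParentEnemy_Child is an enemy NPC variant that inherits its behavior from a parent enemy Blueprint.
; On BeginPlay it runs the parent logic, then overrides the damage, cooldown, speed and max health stats.
; It sets current health to max and writes that value to the HP text.
; Overlap, Tick and construction only forward to the parent.
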(event EventBeginPlay
  (|CallParentFunction)
  (Variables|Default|SetDamage 8.0)
  (Variables|Default|SetCooldown 3.0)
  (Variables|Default|SetSpeed 4.5)
  (bind _output_get (Variables|Default|SetMaxHealt 1.2e+02))
  (bind _output_get_2 (Variables|Default|SetCurrentHealt _output_get))
  (Rendering|Components|TextRender|SetText (Variables|Default|GetHP) (Utilities|Text|ToText(Float) _output_get_2 "HalfToEven")))

(event Collision|EventActorBeginOverlap
  (params (OtherActor :type Actor%20Object%20Reference))
  (|CallParentFunction OtherActor))

(event EventTick
  (params (DeltaSeconds :type Float%20%28single-precision%29))
  (|CallParentFunction DeltaSeconds))

(fn ConstructionScript
  (|CallParentFunction))