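; Enemy spawner actor that spawns queued enemy classes one after another at its own transform.
; BeginPlay sets a one-shot delayed timer targeting SpawnEnemy.
; The SpawnEnemy function spawns and removes the first queue entry, then re-arms a shorter timer by function name, stopping once the queue is empty.
; AddEnemyToQueue only appends, as its immediate spawn branch is unreachable, so it does not restart a stopped chain.
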(event Custom|Spawn%20Enemy)

(event EventBeginPlay
  (Utilities|Time|SetTimerbyEvent (delegate Custom|Spawn%20Enemy) 5.0))

(event Collision|EventActorBeginOverlap
  (params (OtherActor :type Actor%20Object%20Reference)))

(fn ConstructionScript)

(fn SpawnEnemy
  (if (Utilities|Array|IsValidIndex (Variables|Default|GetEnemyQueue))
    (Game|SpawnActorfromClass (Utilities|Array|Get(acopy) (Variables|Default|GetEnemyQueue)) (Transformation|GetActorTransform) "Undefined" "MultiplyWithRoot" 0 0)
    (Utilities|Array|RemoveIndex (Variables|Default|GetEnemyQueue))
    (Utilities|Time|SetTimerbyFunctionName 0 "SpawnEnemy" 2.0)
    (return true)
    (else
      (return false))))

(fn AddEnemytoQueue
  (params (EnemyClass :type BP%20Parent%20Enemy%20Class%20Reference%20%28by%20ref%29))
  (Utilities|Array|Add (Variables|Default|GetEnemyQueue) EnemyClass)
  (if (not true)
    (CallFunction|SpawnEnemy)))