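; BP_Gun_Shotgun is a shotgun weapon Blueprint that handles firing with a short cooldown between shots.
; StartShooting plays the rifle shoot animation on the gun mesh and calls FireShotgun, whose logic lives outside these graphs.
; An IsWaiting flag and a Delay block further shots until the cooldown ends.
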(event EventBeginPlay
  (|CallParentFunction) ; This node is disabled and will not be called.\nDrag off pins to build functionality.
)

(event Collision|EventActorBeginOverlap
  (params (OtherActor :type Actor%20Object%20Reference))
  (|CallParentFunction OtherActor) ; This node is disabled and will not be called.\nDrag off pins to build functionality.
)

(event EventTick
  (params (DeltaSeconds :type Float%20%28single-precision%29))
  (|CallParentFunction DeltaSeconds) ; This node is disabled and will not be called.\nDrag off pins to build functionality.
)

(event EventStartShooting
  (if (not (Variables|Default|GetisWaiting))
    (Components|Animation|PlayAnimation (Variables|Default|GetGunMesh) "/Game/FirstPersonArms/Animations/FP_Rifle_Shoot_Montage.FP_Rifle_Shoot_Montage" false)
    (CallFunction|FireShotgun)
    (Variables|Default|SetisWaiting true)
    (Utilities|FlowControl|Delay 0.5)
    (Variables|Default|SetisWaiting false)))

(fn ConstructionScript
  (|CallParentFunction))