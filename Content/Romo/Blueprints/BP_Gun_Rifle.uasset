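; Rifle gun Blueprint that provides automatic fire between StartShooting and StopShooting.
; StartShooting binds itself to a looping FireRate timer, so each shot re-runs the event and sets the timer again.
; Each run calls FireWeapon, plays a fire sound at the gun mesh and plays the rifle shoot montage on the player's first-person mesh.
; StopShooting clears the stored timer handle to end firing.
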(event EventBeginPlay
  (|CallParentFunction) ; This node is disabled and will not be called.\nDrag off pins to build functionality.
)

(event Collision|EventActorBeginOverlap
  (params (OtherActor :type Actor%20Object%20Reference))
  (|CallParentFunction OtherActor) ; This node is disabled and will not be called.\nDrag off pins to build functionality.
)

(event EventTick
  (params (DeltaSeconds :type Float%20%28single-precision%29))
  (|CallParentFunction DeltaSeconds) ; This node is disabled and will not be called.\nDrag off pins to build functionality.
)

(event EventStartShooting
  (bind _returnvalue (Utilities|Time|SetTimerbyEvent (delegate EventStartShooting) (Variables|Default|GetfireRate) true))
  (Variables|Default|SetfireEvent _returnvalue)
  (CallFunction|FireWeapon)
  (Audio|PlaySoundatLocation "/Game/FPWeapon/Audio/FirstPersonTemplateWeaponFire02.FirstPersonTemplateWeaponFire02" (Transformation|GetWorldLocation (Variables|Default|GetGunMesh)) "0, 0, 0" 1.0 1.0 0.0 0 0 0 0)
  (Animation|Montage|MontagePlay (Components|SkeletalMesh|GetAnimInstance (Variables|/Game/Romo/Blueprints/BP_Character.BP_Character_C|GetFirstPersonMesh (Variables|Default|GetPlayerReference))) "/Game/FirstPersonArms/Animations/FP_Rifle_Shoot_Montage.FP_Rifle_Shoot_Montage" 1.0 "MontageLength" 0.0 true))

(event EventStopShooting
  (Utilities|Time|ClearandInvalidateTimerbyHandle (Variables|Default|GetfireEvent)))

(fn ConstructionScript
  (|CallParentFunction))