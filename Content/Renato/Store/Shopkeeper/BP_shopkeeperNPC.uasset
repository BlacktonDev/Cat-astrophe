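; Shopkeeper NPC that opens the store UI when the player walks into its trigger during the pre-round phase.
; On ShopTrigger overlap it checks InPreRound on BP_FirstPersonGameMode, then creates UI_Shopkeeper with a reference to itself.
; It switches input to UI only, shows the cursor, blends the camera to the NPC and hides the player character.
; Outside pre-round it only prints a refusal, and nothing here reverses the shop state.
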(event OnComponentBeginOverlap(ShopTrigger)
  (params (OverlappedComponent :type Primitive%20Component%20Object%20Reference) (OtherActor :type Actor%20Object%20Reference) (OtherComp :type Primitive%20Component%20Object%20Reference) (OtherBodyIndex :type Integer) (bFromSweep :type Boolean) (SweepResult :type Hit%20Result%20Structure%20%28by%20ref%29))
  (bind _returnvalue (Game|GetPlayerController 0))
  (bind _asbp_first_person_game_mode (Utilities|Casting|CastToBP_FirstPersonGameMode (Game|GetGameMode))
    (:then
      (if (Variables|/Game/Romo/Blueprints/BP_FirstPersonGameMode.BP_FirstPersonGameMode_C|GetInPreRound _asbp_first_person_game_mode)
        (if (== OtherActor (Game|GetPlayerCharacter 0)) ; Ideally set movement speed to 0 at this time or add interaction button to fix displacemment, or a wall
          (bind _returnvalue_2 (UserInterface|CreateWidget "/Game/Renato/Store/Shopkeeper/UI_Shopkeeper.UI_Shopkeeper_C" 0 self))
          (Input|SetInputModeUIOnly _returnvalue _returnvalue_2 "DoNotLock" false)
          (Game|Player|SetViewTargetwithBlend (Game|GetPlayerController 0) self 0.25 "VTBlend_Linear" 0.0 false)
          (UserInterface|Viewport|AddtoViewport _returnvalue_2 0)
          (Variables|/Script/Engine.PlayerController|SetbShowMouseCursor _returnvalue true)
          (Rendering|SetActorHiddenInGame (Game|GetPlayerCharacter 0) true))
        (else
          (Development|PrintString "Cant buy"))))
    (:CastFailed
      (Development|PrintString "No sirve tu chingadera"))))

(fn ConstructionScript)