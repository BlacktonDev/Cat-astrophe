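; BP_DropParent is a loot drop pickup that grants a random buff to the player and destroys itself after five seconds if untouched.
; When a Player-tagged actor overlaps its Sphere, it destroys itself, then randomly picks a speed boost, full heal or nuke cast on BP_Character, with nuke least likely.
; The speed boost's revert follows a Delay on the already destroyed pickup, so it likely never runs.
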(event OnComponentBeginOverlap(Sphere)
  (params (OverlappedComponent :type Primitive%20Component%20Object%20Reference) (OtherActor :type Actor%20Object%20Reference) (OtherComp :type Primitive%20Component%20Object%20Reference) (OtherBodyIndex :type Integer) (bFromSweep :type Boolean) (SweepResult :type Hit%20Result%20Structure%20%28by%20ref%29))
  (bind _returnvalue (Game|GetPlayerCharacter 0))
  (if (Actor|ActorHasTag OtherActor "Player")
    (Actor|DestroyActor)
    (switch int (Math|Random|RandomInteger 5)
      (:0
        (Development|PrintString "MS buff" :!label _label)
        (bind _asbp_character (Utilities|Casting|CastToBP_Character _returnvalue))
        (Variables|/Script/Engine.CharacterMovementComponent|SetMaxWalkSpeed (Variables|/Script/Engine.Character|GetCharacterMovement _asbp_character) 1.2e+03)
        (Variables|/Game/Romo/Blueprints/BP_Character.BP_Character_C|SetSprintSpeed _asbp_character 2e+03)
        (Utilities|FlowControl|Delay 1e+01)
        (Variables|/Script/Engine.CharacterMovementComponent|SetMaxWalkSpeed (Variables|/Script/Engine.Character|GetCharacterMovement _asbp_character) 6e+02)
        (Variables|/Game/Romo/Blueprints/BP_Character.BP_Character_C|SetSprintSpeed _asbp_character 1e+03))
      (:1
        (goto _label))
      (:2
        (Development|PrintString "Heal" :!label _label_2)
        (bind _asbp_character_2 (Utilities|Casting|CastToBP_Character _returnvalue))
        (Variables|/Game/Romo/Blueprints/BP_Character.BP_Character_C|SetCurrentHealt _asbp_character_2 1e+02))
      (:3
        (goto _label_2))
      (:4
        (Development|PrintString "NUKE")
        (bind _asbp_character_3 (Utilities|Casting|CastToBP_Character _returnvalue))
        (Default|NukeCast _asbp_character_3)))))

(event EventBeginPlay
  (Components|Activation|Activate (Variables|Default|GetSphere) false)
  (Utilities|FlowControl|Delay 5.0)
  (Actor|DestroyActor))

(fn ConstructionScript)